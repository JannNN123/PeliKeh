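; Collectible pickup that restores the player character's Lifeforce when it overlaps the Box trigger.
; It matches the overlapping actor by display name "BB_Mycaracter", then casts it to that class.
; If Lifeforce is below full, it adds an amount scaled by elapsed game time and the Efect variable, capped at full.
; The collectible is never destroyed or disabled here, so each new overlap applies the effect again.
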(event OnComponentBeginOverlap(Box)
  (params (OverlappedComponent :type Primitive%20Component%20Object%20Reference) (OtherActor :type Actor%20Object%20Reference) (OtherComp :type Primitive%20Component%20Object%20Reference) (OtherBodyIndex :type Integer) (bFromSweep :type Boolean) (SweepResult :type Hit%20Result%20Structure%20%28by%20ref%29))
  (if (Utilities|Enum|Equal(Enum) (Utilities|GetDisplayName OtherActor) "BB_Mycaracter")
    (bind _asbb_mycaracter (Utilities|Casting|CastToBB_Mycaracter OtherActor))
    (if (< (Variables|/Game/Blueprints/BB_Mycaracter.BB_Mycaracter_C|GetLifeforce _asbb_mycaracter) 1.0)
      (if (<= (+ (Variables|/Game/Blueprints/BB_Mycaracter.BB_Mycaracter_C|GetLifeforce _asbb_mycaracter) (* (/ (Utilities|Time|GetGameTimeinSeconds) 5.0) (Variables|Default|GetEfect))) 1.0)
        (Variables|/Game/Blueprints/BB_Mycaracter.BB_Mycaracter_C|SetLifeforce _asbb_mycaracter (+ (Variables|/Game/Blueprints/BB_Mycaracter.BB_Mycaracter_C|GetLifeforce _asbb_mycaracter) (* (/ (Utilities|Time|GetGameTimeinSeconds) 5.0) (Variables|Default|GetEfect))))
        (else
          (Variables|/Game/Blueprints/BB_Mycaracter.BB_Mycaracter_C|SetLifeforce _asbb_mycaracter 1.0))))))

(fn ConstructionScript)

(fn NewFunction0)