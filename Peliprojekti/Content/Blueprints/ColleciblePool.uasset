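; Actor that acts as a collectible pool, spawning Collectible actors up to a maximum count.
; CreateCollectible spawns one at a set start X and random Z, then stores it in ThePool and increments the count.
; It also rerolls its own Speed variable within bounds derived from the current Speed and elapsed game time.
; UpdateCollectible is an empty stub, and nothing here calls creation or recycles pooled actors.
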(event EventBeginPlay)

(event Collision|EventActorBeginOverlap
  (params (OtherActor :type Actor%20Object%20Reference)))

(event EventTick
  (params (DeltaSeconds :type Float%20%28single-precision%29)))

(fn ConstructionScript)

(fn CreateCollectible
  (if (< (Variables|Default|GetnumberofCollectible) (Variables|Default|GetmaxNumberofCollectible))
    (bind _returnvalue (Game|SpawnActorfromClass "/Game/Blueprints/Collectible.Collectible_C" (Math|Transform|MakeTransform (Math|Vector|MakeVector (Variables|Default|GetcollectibleStartX) 0.0 (Math|Random|RandomFloatinRange -4e+02 1e+03))) "Undefined" 0 0))
    (Variables|Default|SetSpeed (Math|Random|RandomFloatinRange (/ (Variables|UserOptions|Basic|GetSpeed) (/ (Utilities|Time|GetGameTimeinSeconds) 1e+01)) (Variables|UserOptions|Basic|GetSpeed)))
    (Utilities|Array|Insert (Variables|Default|GetthePool) _returnvalue (Variables|Default|GetnumberofCollectible))
    (Math|Integer|IncrementInt (Variables|Default|GetnumberofCollectible))))

(fn UpdateCollectible)